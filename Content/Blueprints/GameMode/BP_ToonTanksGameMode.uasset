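; BP_ToonTanksGameMode is the game mode Blueprint that puts up the UI for the start and end of a Toon Tanks match.
; StartGame creates and adds the start game widget and the gold widget to the viewport.
; GameOver shows the end game widget and sets its display text to a won or lost message based on WonGame.
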(event EventBeginPlay)

(event EventTick
  (params (DeltaSeconds :type Float%20%28single-precision%29)))

(event EventStartGame
  (bind _returnvalue (UserInterface|CreateWidget "/Game/Blueprints/Widgets/WBP_StartGameWidget.WBP_StartGameWidget_C"))
  (UserInterface|Viewport|AddtoViewport _returnvalue 0)
  (bind _returnvalue_2 (UserInterface|CreateWidget "/Game/Blueprints/Widgets/WBP_Gold.WBP_Gold_C"))
  (UserInterface|Viewport|AddtoViewport _returnvalue_2 0))

(event EventGameOver
  (params (bWonGame :type Boolean))
  (bind _returnvalue (UserInterface|CreateWidget "/Game/Blueprints/Widgets/WBP_EndGameWidget.WBP_EndGameWidget_C"))
  (UserInterface|Viewport|AddtoViewport _returnvalue 0)
  (if bWonGame
    (Rendering|Components|TextRender|SetText (Variables|/Game/Blueprints/Widgets/WBP_EndGameWidget.WBP_EndGameWidget_C|GetDisplayText _returnvalue) "Won Game!")
    (else
      (Rendering|Components|TextRender|SetText (Variables|/Game/Blueprints/Widgets/WBP_EndGameWidget.WBP_EndGameWidget_C|GetDisplayText _returnvalue) "Lost Game!"))))

(fn ConstructionScript)